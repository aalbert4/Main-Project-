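; Player controller that handles swipe-to-cut input for rope links.
; Holding CutPress sets the cutting state, and releasing it processes the swipe points, then clears them.
; ProcessSwipe runs multi-sphere traces on the Visibility channel between consecutive points and calls CutAtLink on hit BP_RopeLink actors.
; Tick checks the sample interval while cutting, but that branch is empty, so no points are recorded here.
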(event EventTick
  (params (DeltaSeconds :type Float%20%28single-precision%29))
  (if (Variables|Default|GetbISCutting)
    (if (>= (- (Utilities|Time|GetGameTimeinSeconds) (Variables|Default|GetLastSampleTime)) (Variables|Default|GetSampleInterval))
      _)))

(event Input|ActionEvents|InputActionCutPress
  (params (Key :type Key%20Structure :default "None"))
  (:Pressed
    (Variables|Default|SetbISCutting true)
    (Utilities|Array|Clear (Variables|Default|GetSwipePoints))
    (Variables|Default|SetLastSampleTime -999.0))
  (:Released
    (CallFunction|ProcessSwipe (Variables|Default|GetSwipePoints))
    (Variables|Default|SetbISCutting false)
    (Utilities|Array|Clear (Variables|Default|GetSwipePoints))))

(fn ConstructionScript)

(fn ProcessSwipe
  (params (Points :type Array%20of%20Vectors))
  (bind _returnvalue (Utilities|Array|Length Points))
  (if (>= _returnvalue 2)
    (for _index (range 0 (- _returnvalue 2))
      (bind _outhits (Collision|MultiSphereTraceByChannel (Utilities|Array|Get(acopy) Points _index) (Utilities|Array|Get(acopy) Points (+ _index 1)) (Variables|Default|GetSwipeRadius) "TraceTypeQuery1" false (Utilities|Array|MakeArray self) "None"))
      (for _array_element _outhits
        (bind _asbp_rope_link (Utilities|Casting|CastToBP_RopeLink (.HitActor (Collision|BreakHitResult _array_element))))
        (Default|CutatLink _asbp_rope_link)))
    (return)
    (else
      (return))))