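; BP_RopeLink is a single rope segment actor with a collider and references to constraints toward its previous and next links.
; CutAtLink severs the rope at this segment by destroying both constraints when valid.
; SetupConstriant, called on BeginPlay without a link to join, is unfinished: it only fetches the other link's collider for a previous link.
; Its constraint assignment and component-linking nodes are disconnected and never run.
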(event EventBeginPlay
  (CallFunction|SetupConstriant 0 false))

(event Collision|EventActorBeginOverlap
  (params (OtherActor :type Actor%20Object%20Reference)))

(event EventTick
  (params (DeltaSeconds :type Float%20%28single-precision%29)))

(fn ConstructionScript)

(fn CutatLink
  (Utilities|FlowControl|Sequence
    (:then_0
      (Utilities|IsValid (Variables|Default|GetConstraintToPrevious)
        (:Is%20Valid
          (if true
            (Components|DestroyComponent (Variables|Default|GetConstraintToPrevious))))))
    (:then_1
      (Utilities|IsValid (Variables|Default|GetConstraintToNext)
        (:Is%20Valid
          (if true
            (Components|DestroyComponent (Variables|Default|GetConstraintToNext))))))))

(fn SetupConstriant
  (params (OtherLink :type BP%20Rope%20Link%20Object%20Reference) (bIsPrev :type Boolean))
  (Utilities|IsValid OtherLink
    (:Is%20Valid
      (if bIsPrev
        (bind _collider (CallFunction|GetCollider OtherLink))))))

(fn GetCollider
  (return (Variables|Default|GetCollider)))