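; Rope actor meant to build a vertical chain of BP_RopeLink child actors below its Anchor on BeginPlay, then print the link count.
; BuildRope spaces links by LinkSpacing, sets previous/next references and calls each link's SetupConstriant against its predecessor.
; As wired, spawning runs inside the old-component cleanup loop, both arrays are cleared afterwards, and the node recording new components is unconnected.
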(event EventBeginPlay
  (CallFunction|BuildRope)
  (Development|PrintString (Utilities|String|Append (Utilities|String|MakeLiteralString "Links") (Utilities|String|ToString(Integer) (Utilities|Array|Length (Variables|Default|GetLinks))))))

(event Collision|EventActorBeginOverlap
  (params (OtherActor :type Actor%20Object%20Reference)))

(event EventTick
  (params (DeltaSeconds :type Float%20%28single-precision%29)))

(fn ConstructionScript)

(fn BuildRope
  (bind _links (Variables|Default|GetLinks))
  (bind _returnvalue (Utilities|Array|Length _links))
  (for _array_element (Variables|Default|GetChildLinkComponents)
    (Utilities|IsValid _array_element
      (:Is%20Valid
        (if true
          (Components|DestroyComponent _array_element)
          (for _index (range 0 (- (Variables|Default|GetNumLinks) 1))
            (bind _returnvalue_2 (AddComponent|AddChildActorComponent (Variables|Default|GetLinkClass) false))
            (Transformation|SetWorldLocation _returnvalue_2 (+ (Transformation|GetWorldLocation (Variables|Default|GetAnchor)) (Math|Vector|MakeVector 0.0 0.0 (* (* (Variables|Default|GetLinkSpacing) _index) -1.0))) false false)
            (bind _asbp_rope_link (Utilities|Casting|CastToBP_RopeLink (Variables|/Script/Engine.ChildActorComponent|GetChildActor _returnvalue_2)))
            (Utilities|Array|Add (Variables|Default|GetLinks) _asbp_rope_link))
          (if (> _returnvalue 1)
            (for _index_2 (range 1 (- _returnvalue 1))
              (Variables|/Game/Blueprint/BP_RopeLink.BP_RopeLink_C|SetPreviousLink (Utilities|Array|Get(acopy) (Variables|Default|GetLinks) _index_2) (Utilities|Array|Get(acopy) (Variables|Default|GetLinks) (- _index_2 1)))
              (Variables|/Game/Blueprint/BP_RopeLink.BP_RopeLink_C|SetNextLink (Utilities|Array|Get(acopy) (Variables|Default|GetLinks) (- _index_2 1)) (Utilities|Array|Get(acopy) (Variables|Default|GetLinks) _index_2))
              (Default|SetupConstriant (Utilities|Array|Get(acopy) (Variables|Default|GetLinks) _index_2) (Utilities|Array|Get(acopy) (Variables|Default|GetLinks) (- _index_2 1)) true)))))))
  (Utilities|Array|Clear (Variables|Default|GetChildLinkComponents))
  (Utilities|Array|Clear (Variables|Default|GetLinks)))