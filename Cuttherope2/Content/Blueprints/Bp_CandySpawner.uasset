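; Spawner actor for a candy-catching game that drops one BP_Candy at a time from a random Y position at a fixed height.
; It binds each candy's caught and missed events to adjust score and lives, play sounds, update UI through BP_LevelController and spawn the next candy.
; Fall speed rises with score up to a clamp.
; Running out of lives triggers game over, disables player input and stops the music.
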(event Custom|HandleCandyCaught
  (bind _output_get (Variables|Default|SetScore (+ (Variables|Default|GetScore) 10)))
  (Default|UpdateScoreonUI (Variables|Default|GetLevelController) _output_get)
  (Utilities|FlowControl|Delay 0.5)
  (CallFunction|Spawnanddrop)
  (Audio|PlaySound2D "/Game/Audios/monster_chewing.monster_chewing" 1.0 1.0 0.0 0 0))

(event Custom|HandleCandyMissed
  (bind _levelcontroller (Variables|Default|GetLevelController))
  (bind _output_get (Variables|Default|SetCurrentLives (- (Variables|Default|GetCurrentLives) 1)))
  (Default|UpdateLivesonUi (Variables|Default|GetLevelController) _output_get)
  (bind _output_get_2 (Variables|Default|SetScore (- (Variables|Default|GetScore) 10)))
  (Default|UpdateScoreonUI (Variables|Default|GetLevelController) _output_get_2)
  (Audio|PlaySound2D (Variables|Default|GetCandyBreakSound) 1.0 1.0 0.0 0 0)
  (if (< (Variables|Default|GetCurrentLives) 1)
    (Variables|Default|SetGameOver true)
    (Default|ShowGameOveronUI _levelcontroller)
    (Input|DisableInput (Game|Player|GetPlayerPawn 0) (Game|GetPlayerController 0))
    (Default|StopMusic _levelcontroller)
    (else
      (Utilities|FlowControl|Delay 0.2)
      (CallFunction|Spawnanddrop))))

(event EventBeginPlay
  (bind _returnvalue (Actor|GetActorOfClass "/Game/Blueprints/BP_LevelController.BP_LevelController_C"))
  (Variables|Default|SetLevelController _returnvalue)
  (Variables|Default|SetCurrentLives (Variables|Default|GetMaxLives))
  (Utilities|FlowControl|Delay 3.0)
  (CallFunction|Spawnanddrop))

(fn ConstructionScript)

(fn GetRandomSpawnLoc
  (return (Math|Vector|MakeVector 0.0 (Math|Random|RandomFloatinRange (Variables|Default|GetMinY) (Variables|Default|GetMaxY)) (Variables|Default|GetTopZ))))

(fn BindCandy
  (params (Candy :type BP%20Candy%20Object%20Reference))
  (EventDispatchers|BindEventtoOnCandyCaught Candy (EventDispatchers|CreateEvent :!event Custom|HandleCandyCaught))
  (EventDispatchers|BindEventtoOnCandyMissed Candy (EventDispatchers|CreateEvent :!event Custom|HandleCandyMissed)))

(fn Spawnanddrop
  (bind _basefallspeed (Variables|Default|GetBaseFallSpeed))
  (if (Variables|Default|GetGameOver)
    (return)
    (else
      (bind _spawnloc (CallFunction|GetRandomSpawnLoc))
      (bind _returnvalue (Game|SpawnActorfromClass "/Game/Blueprints/BP_Candy.BP_Candy_C" (Math|Transform|MakeTransform _spawnloc "0.000000,90.000000,0.000000") "AlwaysSpawn" "MultiplyWithRoot" 0 0))
      (Variables|Default|SetCandyClass _returnvalue)
      (Variables|/Game/Blueprints/BP_Candy.BP_Candy_C|SetFallSpeed _returnvalue (Math|Float|Clamp(Float) (+ _basefallspeed (* (Variables|Default|GetSpeedPerHit) (Math|Conversions|ToFloat(Integer) (/ (Variables|Default|GetScore) 10)))) _basefallspeed (Variables|Default|GetMaxFallSpeed)))
      (CallFunction|BindCandy _returnvalue)
      (Default|DropCandy _returnvalue _spawnloc))))