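; BP_LevelController runs level-wide game flow, handling the HUD, background music and restarting after game over.
; On BeginPlay it enables player input, creates BP_UserWidget and starts the music, which cycles through MusicTracks whenever a track finishes.
; Its functions and events forward score, lives, special-effect state and game over to the widget.
; Once GameOver is set, the Restart Game input reloads MainGameLevel.
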(event OnAudioFinished(MusicAudio)
  (CallFunction|PlayNextTrack))

(event Custom|SetSpeciialActiveOnUi
  (params (IsActive :type Boolean))
  (bind _mainui (Variables|Default|GetMainUi))
  ;[1 1 1] Greenish special effect for player
  (Utilities|IsValid _mainui
    (:Is%20Valid
      (Default|SetSpecialActive _mainui IsActive))))

(event EventBeginPlay
  (bind _returnvalue (Game|GetPlayerController 0))
  ;[1 1 1] Gane Start Logic
  (Input|EnableInput _returnvalue)
  (bind _returnvalue_2 (UserInterface|CreateWidget "/Game/Blueprints/BP_UserWidget.BP_UserWidget_C" _returnvalue))
  (bind _output_get (Variables|Default|SetMainUi _returnvalue_2))
  (UserInterface|Viewport|AddtoViewport _output_get 0)
  (CallFunction|PlayNextTrack))

(event Input|ActionEvents|InputActionRestartGame
  (params (Key :type Key%20Structure :default "None"))
  ;[1 1 1] Restarting Game once game is over
  (:Pressed
    (if (Variables|Default|GetGame%20Over?)
      (Game|OpenLevel(byName) "MainGameLevel"))))

(fn ConstructionScript)

(fn UpdateScoreonUI
  (params (NewScore :type Integer))
  (bind _mainui (Variables|Default|GetMainUi))
  (Utilities|IsValid _mainui
    (:Is%20Valid
      (Default|UpdateScore _mainui NewScore))))

(fn PlayNextTrack
  (bind _music_tracks (Variables|Default|GetMusic%20Tracks))
  (bind _musicaudio (Variables|Default|GetMusicAudio))
  (bind _returnvalue (Utilities|Array|Length _music_tracks))
  (if (<= _returnvalue 0)
    (return)
    (else
      (bind _output_get (Variables|Default|SetCurrentTrackIndex (Math|Integer|%(Integer) (+ (Variables|Default|GetCurrentTrackIndex) 1) _returnvalue)))
      (Audio|Components|Audio|SetSound _musicaudio (Utilities|Array|Get(acopy) (Variables|Default|GetMusic%20Tracks) _output_get))
      (Audio|Components|Audio|Play _musicaudio 0.0)
      (return))))

(fn UpdateLivesonUi
  (params (Newlives :type Integer))
  (bind _mainui (Variables|Default|GetMainUi))
  (Utilities|IsValid _mainui
    (:Is%20Valid
      (if true
        (Default|UpdateLives _mainui Newlives)
        (else
          (return))))))

(fn ShowGameOveronUI
  (Default|GameOver (Variables|Default|GetMainUi))
  (Variables|Default|SetGame%20Over? true))

(fn StopMusic
  (Audio|Components|Audio|Stop (Variables|Default|GetMusicAudio)))