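; BP_OmNom is the player-moved Om Nom character that catches falling or placed candy with its mouth.
; An input axis slides it along world Y with a swept, frame-rate-independent move clamped between limits.
; Overlaps on MouthTrigger call Caught on any BP_Candy.
; PlayEatAnimation and PlayThrowupAnimation events play one-shot Paper2D flipbooks, each guarded by its own flag, and OnFinishedPlaying switches back to idle.
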(event OnComponentBeginOverlap(MouthTrigger)
  (params (OverlappedComponent :type Primitive%20Component%20Object%20Reference) (OtherActor :type Actor%20Object%20Reference) (OtherComp :type Primitive%20Component%20Object%20Reference) (OtherBodyIndex :type Integer) (bFromSweep :type Boolean) (SweepResult :type Hit%20Result%20Structure%20%28by%20ref%29))
  (bind _asbp_candy (Utilities|Casting|CastToBP_Candy OtherActor))
  (Default|Caught _asbp_candy))

(event OnFinishedPlaying(PaperFlipbook)
  (bind _paperflipbook (Variables|Default|GetPaperFlipbook))
  ;[1 1 1] Idle animation
  (if (Variables|Default|GetisEating)
    (Sprite|SetFlipbook _paperflipbook (Variables|Default|GetIdleFlipbook))
    (Audio|Components|Audio|Play _paperflipbook)
    (Variables|Default|SetisEating false)
    (elif (Variables|Default|GetisThrowingUp)
      (Sprite|SetFlipbook _paperflipbook (Variables|Default|GetIdleFlipbook))
      (Audio|Components|Audio|Play _paperflipbook)
      (Variables|Default|SetisThrowingUp false))))

(event Custom|PlayEatAnimation
  (bind _paperflipbook (Variables|Default|GetPaperFlipbook))
  ;[1 1 1] Omnom eat annimation
  (if (not (Variables|Default|GetisEating))
    (Variables|Default|SetisEating true)
    (Components|Timeline|SetLooping _paperflipbook false)
    (Sprite|SetFlipbook _paperflipbook (Variables|Default|GetEatFlipbook))
    (Components|Timeline|PlayfromStart _paperflipbook)))

(event Custom|PlayThrowupAnimation
  (bind _paperflipbook (Variables|Default|GetPaperFlipbook))
  ;[1 1 1] Throwup Animation
  (if (not (Variables|Default|GetisThrowingUp))
    (Variables|Default|SetisThrowingUp true)
    (Components|Timeline|SetLooping _paperflipbook false)
    (Sprite|SetFlipbook _paperflipbook (Variables|Default|GetThrowupFlipbook))
    (Components|Timeline|PlayfromStart _paperflipbook)))

(event Input|AxisEvents|InputAxisMoveRIght
  (params (AxisValue :type Float%20%28single-precision%29))
  (bind _returnvalue (Transformation|GetActorLocation))
  (bind (_x _y _z) (Math|Vector|BreakVector _returnvalue))
  ;[1 1 1] Move Physics
  (if (> (Math|Float|Absolute(Float) AxisValue) 0.01)
    (Transformation|SetActorLocation (Math|Vector|MakeVector _x (Math|Float|Clamp(Float) (+ _y (* (* (* (Variables|Default|GetMoveSpeed) AxisValue) (Variables|Default|GetSpeedMultiplier)) (Utilities|Time|GetWorldDeltaSeconds))) (Variables|Default|GetMinX) (Variables|Default|GetMaxX)) _z) true false)))

(fn ConstructionScript)