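; BP_Candy is a falling candy actor that can be caught or missed.
; DropCandy moves it to a spawn location, reveals its sprite and starts physics with gravity and an initial downward velocity from FallSpeed.
; While dropped, Tick calls Missed once the actor's height falls below MissZ; Caught is exposed as a separate function.
; Both outcomes stop physics, fire their caught or missed dispatcher and destroy the actor.
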(event EventTick
  (params (DeltaSeconds :type Float%20%28single-precision%29))
  (if (Variables|Default|GetIsDropped)
    (if (< (.Z (Math|Vector|BreakVector (Transformation|GetActorLocation))) (Variables|Default|GetMissZ))
      (CallFunction|Missed))))

(fn ConstructionScript)

(fn DropCandy
  (params (SpawnLoc :type Vector))
  (bind _candysprite (Variables|Default|GetCandySprite))
  (bind _candysprite_2 (Variables|Default|GetCandySprite))
  (Transformation|SetActorLocation SpawnLoc false false)
  (Development|SetHiddeninGame _candysprite false false)
  (Physics|SetSimulatePhysics _candysprite_2 true)
  (Physics|SetEnableGravity _candysprite_2 true)
  (Physics|SetPhysicsLinearVelocity _candysprite (Math|Vector|MakeVector 0.0 0.0 (* (Variables|Default|GetFallSpeed) -1.0)) false "None")
  (Variables|Default|SetIsDropped true))

(fn Caught
  (bind _candysprite (Variables|Default|GetCandySprite))
  (if (Variables|Default|GetIsDropped)
    (Variables|Default|SetIsDropped false)
    (Physics|SetSimulatePhysics _candysprite false)
    (Development|SetHiddeninGame _candysprite true false)
    (Default|CallOnCandyCaught)
    (Actor|DestroyActor)
    (else
      (return))))

(fn Missed
  (if true
    (Variables|Default|SetIsDropped false)
    (Physics|SetSimulatePhysics (Variables|Default|GetCandySprite) false)
    (Default|CallOnCandyMissed)
    (Actor|DestroyActor)
    (else
      (return))))